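; Main mod Blueprint that adds a noclip fly mode and a detachable free camera for the player.
; Tick polls hardcoded keys: F5 toggles flying without capsule collision, with offset-based vertical movement and a Shift forward boost.
; F4 alternates possession between the original pawn and a lazily spawned, hidden, collisionless DefaultPawn.
; While in free camera, Shift raises speed through a FloatingPawnMovement component added at runtime.
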(event EventTick
  (params (DeltaSeconds :type Float%20%28single-precision%29))
  ;[1 1 1 1 15] The codes are a mess but it works..
  (Utilities|FlowControl|Sequence
    (:then_0
      (Utilities|FlyToggle))
    (:then_1
      (Utilities|FreeCameraToggle))))

(fn ConstructionScript
  (|CallParentFunction))

(fn ModButtonWasPressed
  (params (FunctionIndex :type Integer))
  (switch int FunctionIndex))